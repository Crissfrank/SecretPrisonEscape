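; Laser beam actor that shows a colored beam and chains into bounced lasers on reflectors.
; Each tick it box-traces along its up vector and stretches its mesh to the hit distance or full range.
; Target changes go through BPI_Lasers and SpawnRef to create or remove follow-on lasers, while a steady BPC_Reflect hit repositions and rotates the bounce laser.
; CancelTargetHit releases or deactivates the last target and destroys the beam unless overridden.
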(event `self.ReceiveBeginPlay`
  (`self.Change Color`))

(event `self.ReceiveTick`
  (params (DeltaSeconds :type "Float (single-precision)"))
  (`self.Set End Position`))

(fn `Cancel Target Hit`
  (params (Override :type Boolean))
  (returns (`Remove from Array` :type Boolean))
  (`|ExecutionSequence`
    (:`then_0`
      (bind _lasthitactor (`self.LastHitActor`)
        (:`then`
          (bind _asbp_laser_parent (cast `/Game/MeinZeug/BluePrints/Laser/BP_LaserParent` _lasthitactor))
          (if (and (`KismetSystemLibrary.DoesImplementInterface` _asbp_laser_parent "/Game/MeinZeug/BluePrints/Interfaces/BPI_Lasers.BPI_Lasers_C") (`KismetArrayLibrary.Array_IsEmpty` (`/Game/MeinZeug/BluePrints/Laser/BP_LaserParent.LaserAttached` _asbp_laser_parent)))
            (message `/Game/MeinZeug/BluePrints/Interfaces/BPI_Lasers.LaserBounce` (`self.LastHitActor`) false (struct) self)
            (else
              (set `/Game/MeinZeug/BluePrints/Laser/BP_LaserParent.Active` false _asbp_laser_parent))))
        (:`else`)))
    (:`then_1`
      (if (`local.Override`)
        (return false)
        (else
          (`self.K2_DestroyActor`)
          (return true))))))

(fn `Change Color`
  (bind _returnvalue (`PrimitiveComponent.CreateDynamicMaterialInstance` (`self.SM_Parent`) 0 "/Game/MeinZeug/Materials/SpecialMats/M_Laser.M_Laser" "None"))
  (`MaterialInstanceDynamic.SetVectorParameterValue` _returnvalue "Color" (`self.LaserColor`)))

(fn `Set End Position`
  (locals (Range :type "Float (double-precision)" :default 3000.0) (`Hit Info` :type "HitResult Structure") (HitActor :type "Actor Object Reference"))
  (bind _returnvalue (`self.GetActorUpVector`))
  (bind (_bblockinghit _binitialoverlap _time _distance _location _impactpoint _normal _impactnormal _physmat _hitactor _hitcomponent _hitbonename _bonename _hititem _elementindex _faceindex _tracestart) (`GameplayStatics.BreakHitResult` (`local.Hit Info`)))
  (bind _returnvalue_2 (+ (`self.K2_GetActorLocation`) (* _returnvalue 2.0)))
  (bind _outhit (`KismetSystemLibrary.BoxTraceSingle` _returnvalue_2 (+ _returnvalue_2 (* _returnvalue (`local.Range`))) (0.5 0.5 0.5) (struct) "TraceTypeQuery1"))
  (bind _output_get (set `local.Hit Info` _outhit))
  (bind (_bblockinghit_2 _binitialoverlap_2 _time_2 _distance_2 _location_2 _impactpoint_2 _normal_2 _impactnormal_2 _physmat_2 _hitactor_2) (`GameplayStatics.BreakHitResult` _output_get))
  (set `local.HitActor` _hitactor_2)
  (`SceneComponent.SetWorldScale3D` (`self.SM_Parent`) (`KismetMathLibrary.MakeVector` 0.05 0.05 (`KismetMathLibrary.SelectFloat` (/ (+ _distance_2 1.0) 100.0) (/ (`local.Range`) 100.0) _bblockinghit_2)))
  (`local.HitActor`
    (:`then`
      (`|ExecutionSequence`
        (:`then_0`
          (if (== (`self.LastHitActor`) (`local.HitActor`))
            (bind _asbpc_reflect (cast `/Game/MeinZeug/BluePrints/Laser/BPC_Reflect` (`self.LastHitActor`)))
            (`self.K2_SetActorLocation` (`self.Bounce Laser`) (`.ImpactPoint` (`GameplayStatics.BreakHitResult` (`local.Hit Info`))) false false)
            (`self.K2_SetActorRotation` (`self.Bounce Laser`) (`/Game/MeinZeug/BluePrints/Laser/BPC_Reflect.Calculate Rotation` _asbpc_reflect _impactpoint _impactnormal _tracestart) false)
            (else
              (`|ExecutionSequence`
                (:`then_0`
                  (if (`KismetSystemLibrary.DoesImplementInterface` (`self.LastHitActor`) "/Game/MeinZeug/BluePrints/Interfaces/BPI_Lasers.BPI_Lasers_C")
                    (`/Game/MeinZeug/BluePrints/Laser/BPC_LaserSpawn.Remove Following Lasers` (`self.SpawnRef`) self)))
                (:`then_1`
                  (if (`KismetSystemLibrary.DoesImplementInterface` (`local.HitActor`) "/Game/MeinZeug/BluePrints/Interfaces/BPI_Lasers.BPI_Lasers_C")
                    (bind _new_laser (message `/Game/MeinZeug/BluePrints/Interfaces/BPI_Lasers.LaserBounce` (`local.HitActor`) true (`local.Hit Info`) self))
                    (set `self.Bounce Laser` _new_laser)
                    (`KismetSystemLibrary.PrintString` (`KismetSystemLibrary.GetDisplayName` null))))))))
        (:`then_1`
          (set `self.LastHitActor` (`local.HitActor`)))))
    (:`else`
      (`|ExecutionSequence`
        (:`then_0`
          (bind _lasthitactor (`self.LastHitActor`)
            (:`then`
              (if (`KismetSystemLibrary.DoesImplementInterface` _lasthitactor "/Game/MeinZeug/BluePrints/Interfaces/BPI_Lasers.BPI_Lasers_C")
                (message `/Game/MeinZeug/BluePrints/Interfaces/BPI_Lasers.LaserBounce` (`self.LastHitActor`) true (`local.Hit Info`) self)))
            (:`else`)))
        (:`then_1`
          (set `self.LastHitActor` null)
          (set `self.Bounce Laser` null))))))

(fn `Update ID`
  (params (Append :type String))
  (returns (ReturnValue :type String))
  (return (`KismetStringLibrary.Concat_StrStr` (`self.Laser ID`) Append)))

(fn `UserConstructionScript`
  (`parent.UserConstructionScript`))