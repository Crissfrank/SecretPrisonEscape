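; BPC_LaserSpawn is a laser emitter that spawns and tracks BPC_Laser actors.
; On BeginPlay it spawns the first laser at its Arrow with the actor's rotation, passing color, a self-reference and its display name as LaserID.
; RemoveFollowingLasers walks ChildLaser backwards, using substring ID matching to find a given laser and those following it.
; It calls CancelTargetHit on each, flagging exact matches, and drops those returning true from the array.
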(event `self.ReceiveBeginPlay`
  (set `self.SpawnRef` self)
  (set `self.ID` (`KismetSystemLibrary.GetDisplayName` self))
  (bind _returnvalue (`|SpawnActorFromClass` "/Game/MeinZeug/BluePrints/Laser/BPC_Laser.BPC_Laser_C" (`KismetMathLibrary.MakeTransform` (`SceneComponent.K2_GetComponentLocation` (`self.Arrow`)) (`self.K2_GetActorRotation`)) "Undefined" "MultiplyWithRoot" null (`self.ID`) (`self.LaserColor`) (`self.SpawnRef`) null))
  (`KismetArrayLibrary.Array_Add` (`self.Child Laser`) _returnvalue))

(fn `Remove Following Lasers`
  (params (`Laser Ref` :type "/Game/MeinZeug/BluePrints/Laser/BPC_Laser Object Reference"))
  (locals (`ID Removed` :type String))
  (set `local.ID Removed` (`/Game/MeinZeug/BluePrints/Laser/BPC_Laser.Laser ID` `Laser Ref`))
  (bind (_arrayindex _arrayelement) (`/Engine/EditorBlueprintResources/StandardMacros.ReverseForEachLoop` (`self.Child Laser`))
    (:`LoopBody`
      (`/Engine/EditorBlueprintResources/StandardMacros.IsValid` _arrayelement
        (:`Is Valid`
          (if (`KismetStringLibrary.Contains` (`/Game/MeinZeug/BluePrints/Laser/BPC_Laser.Laser ID` _arrayelement) (`local.ID Removed`))
            (bind _remove_from_array (`/Game/MeinZeug/BluePrints/Laser/BPC_Laser.Cancel Target Hit` _arrayelement (`KismetStringLibrary.EqualEqual_StrStr` (`/Game/MeinZeug/BluePrints/Laser/BPC_Laser.Laser ID` _arrayelement) (`local.ID Removed`))))
            (if _remove_from_array
              (`KismetArrayLibrary.Array_RemoveItem` (`self.Child Laser`) _arrayelement))))))))

(fn `UserConstructionScript`
  (`parent.UserConstructionScript`))