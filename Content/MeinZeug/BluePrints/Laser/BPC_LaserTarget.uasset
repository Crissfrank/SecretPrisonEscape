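; Laser puzzle target that lights up when hit by the laser from its linked origin and counts toward unlocking a door.
; LaserBounce ignores other origins, stores the hit response as Active and passes the laser's color to PuzzleSolved.
; PuzzleSolved tints a dynamic M_Solid material with that color or grey, then increments or decrements DoorToUnlock's IsLaserDone on every call and prints the count.
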(fn `LaserBounce`
  (params (HitResponse :type Boolean) (HitInformation :type "HitResult Structure") (LaserHit :type "/Game/MeinZeug/BluePrints/Laser/BPC_Laser Object Reference") (Origin :type "/Game/MeinZeug/BluePrints/Laser/BPC_LaserSpawn Object Reference"))
  (returns (`New Laser` :type "/Game/MeinZeug/BluePrints/Laser/BPC_Laser Object Reference"))
  (if (== Origin (`self.SpawnRef`))
    (set `self.Active` HitResponse)
    (`self.Puzzle Solved` (`/Game/MeinZeug/BluePrints/Laser/BP_LaserParent.LaserColor` LaserHit))
    (return null)))

(fn `Puzzle Solved`
  (params (`Color Laser` :type "LinearColor Structure"))
  (bind _returnvalue (`PrimitiveComponent.CreateDynamicMaterialInstance` (`self.SM_Parent`) 0 "/Game/LevelPrototyping/Materials/M_Solid.M_Solid" "None"))
  (`MaterialInstanceDynamic.SetVectorParameterValue` _returnvalue "Base Color" (`KismetMathLibrary.SelectColor` `Color Laser` (struct :`R` 0.354167 :`G` 0.354167 :`B` 0.354167 :`A` 1.0) (`self.Active`)))
  (if (`self.Active`)
    (bind _result (`/Engine/EditorBlueprintResources/StandardMacros.IncrementInt` (`/Game/MeinZeug/BluePrints/Laser/BP_LaserDoor.IsLaserDone` (`self.DoorToUnlock`)))
      (:`  `
        (`KismetSystemLibrary.PrintString` (`KismetStringLibrary.Conv_IntToString` _result))))
    (else
      (bind _result_2 (`/Engine/EditorBlueprintResources/StandardMacros.DecrementInt` (`/Game/MeinZeug/BluePrints/Laser/BP_LaserDoor.IsLaserDone` (`self.DoorToUnlock`)))
        (:`  `
          (`KismetSystemLibrary.PrintString` (`KismetStringLibrary.Conv_IntToString` _result_2)))))))

(fn `UserConstructionScript`
  (`parent.UserConstructionScript`))