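; BPC_Reflect is a reflective Blueprint that bounces lasers hitting it.
; On a hit, LaserBounce spawns a BPC_Laser at the impact point along the mirrored direction, inheriting color and source, with an ID updated using "B".
; It records the bounce locally and in the source's child list.
; Without a hit, it destroys its attached lasers whose ID contains the incoming laser's ID.
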(fn `Calculate Rotation`
  (params (`Impact Point` :type "Vector Structure") (`Impact Normal` :type "Vector Structure") (`Trace Start` :type "Vector Structure"))
  (returns (ReturnValue :type "Rotator Structure"))
  (return (`KismetMathLibrary.MakeRotFromZ` (`KismetMathLibrary.MirrorVectorByNormal` (- `Impact Point` `Trace Start`) `Impact Normal`))))

(fn `Clear Attached Lasers`
  (params (`ID Clear` :type String))
  (bind (_arrayindex _arrayelement) (`/Engine/EditorBlueprintResources/StandardMacros.ReverseForEachLoop` (`self.LaserAttached`))
    (:`LoopBody`
      (`/Engine/EditorBlueprintResources/StandardMacros.IsValid` _arrayelement
        (:`Is Valid`
          (if (`KismetStringLibrary.Contains` (`/Game/MeinZeug/BluePrints/Laser/BPC_Laser.Laser ID` _arrayelement) (`local.ID Clear`))
            (`self.K2_DestroyActor` _arrayelement)
            (`KismetArrayLibrary.Array_RemoveItem` (`self.LaserAttached`) _arrayelement)))))))

(fn `LaserBounce`
  (params (HitResponse :type Boolean) (HitInformation :type "HitResult Structure") (LaserHit :type "/Game/MeinZeug/BluePrints/Laser/BPC_Laser Object Reference") (Origin :type "/Game/MeinZeug/BluePrints/Laser/BPC_LaserSpawn Object Reference"))
  (returns (`New Laser` :type "/Game/MeinZeug/BluePrints/Laser/BPC_Laser Object Reference"))
  (bind _laserhit (`local.LaserHit`))
  (bind (_bblockinghit _binitialoverlap _time _distance _location _impactpoint _normal _impactnormal _physmat _hitactor _hitcomponent _hitbonename _bonename _hititem _elementindex _faceindex _tracestart) (`GameplayStatics.BreakHitResult` (`local.HitInformation`)))
  (if (`local.HitResponse`)
    (`KismetSystemLibrary.PrintString` "Hello")
    (bind _returnvalue (`|SpawnActorFromClass` "/Game/MeinZeug/BluePrints/Laser/BPC_Laser.BPC_Laser_C" (`KismetMathLibrary.MakeTransform` _impactpoint (`self.Calculate Rotation` _impactpoint _impactnormal _tracestart)) "AlwaysSpawn" "MultiplyWithRoot" null (`/Game/MeinZeug/BluePrints/Laser/BPC_Laser.Update ID` _laserhit "B") (`/Game/MeinZeug/BluePrints/Laser/BP_LaserParent.LaserColor` _laserhit) (`/Game/MeinZeug/BluePrints/Laser/BP_LaserParent.SpawnRef` _laserhit) null))
    (`KismetSystemLibrary.PrintString` (`KismetSystemLibrary.GetDisplayName` _returnvalue))
    (`KismetArrayLibrary.Array_Add` (`self.LaserAttached`) _returnvalue)
    (`KismetArrayLibrary.Array_Add` (`/Game/MeinZeug/BluePrints/Laser/BPC_LaserSpawn.Child Laser` (`/Game/MeinZeug/BluePrints/Laser/BP_LaserParent.SpawnRef` (`local.LaserHit`))) _returnvalue)
    (return _returnvalue)
    (else
      (`self.Clear Attached Lasers` (`/Game/MeinZeug/BluePrints/Laser/BPC_Laser.Laser ID` (`local.LaserHit`))))))

(fn `UserConstructionScript`
  (`parent.UserConstructionScript`))