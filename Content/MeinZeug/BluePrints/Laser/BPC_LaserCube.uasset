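; Laser puzzle cube that re-emits an incoming laser along its arrow's forward direction and shows a widget while the first-person character is inside its box.
; LaserBounce spawns one child BPC_Laser when first hit, passing on color, spawn reference and an updated ID, then attaches it to SMParent.
; The new beam registers with the cube and the originating SpawnRef; when the hit ends, the cube clears its attached lasers.
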(event `self.Box.OnComponentBeginOverlap`
  (params (OverlappedComponent :type "PrimitiveComponent Object Reference") (OtherActor :type "Actor Object Reference") (OtherComp :type "PrimitiveComponent Object Reference") (OtherBodyIndex :type Integer) (bFromSweep :type Boolean) (SweepResult :type "HitResult Structure (by ref)"))
  (cast `/Game/FirstPerson/Blueprints/BP_FirstPersonCharacter` OtherActor)
  (`SceneComponent.SetHiddenInGame` (`self.Widget`) false false))

(event `self.Box.OnComponentEndOverlap`
  (params (OverlappedComponent :type "PrimitiveComponent Object Reference") (OtherActor :type "Actor Object Reference") (OtherComp :type "PrimitiveComponent Object Reference") (OtherBodyIndex :type Integer))
  (cast `/Game/FirstPerson/Blueprints/BP_FirstPersonCharacter` OtherActor)
  (`SceneComponent.SetHiddenInGame` (`self.Widget`) true false))

(fn `LaserBounce`
  (params (HitResponse :type Boolean) (HitInformation :type "HitResult Structure") (LaserHit :type "/Game/MeinZeug/BluePrints/Laser/BPC_Laser Object Reference") (Origin :type "/Game/MeinZeug/BluePrints/Laser/BPC_LaserSpawn Object Reference"))
  (returns (`New Laser` :type "/Game/MeinZeug/BluePrints/Laser/BPC_Laser Object Reference"))
  (bind _laserhit (`local.LaserHit`))
  (`/Engine/EditorBlueprintResources/StandardMacros.IsValid` LaserHit
    (:`Is Valid`
      (set `self.SpawnRef` (`/Game/MeinZeug/BluePrints/Laser/BP_LaserParent.SpawnRef` LaserHit))
      (if (or (and (`local.HitResponse`) (not (`self.Active`))) (not (`local.HitResponse`)))
        (bind _output_get (set `self.Active` (`local.HitResponse`)))
        (if _output_get
          (bind _returnvalue (`|SpawnActorFromClass` "/Game/MeinZeug/BluePrints/Laser/BPC_Laser.BPC_Laser_C" (`KismetMathLibrary.MakeTransform` (`SceneComponent.K2_GetComponentLocation` (`self.Arrow`)) (`KismetMathLibrary.MakeRotFromZ` (`SceneComponent.GetForwardVector` (`self.Arrow`)))) "Undefined" "MultiplyWithRoot" null (`/Game/MeinZeug/BluePrints/Laser/BPC_Laser.Update ID` _laserhit "C") (`/Game/MeinZeug/BluePrints/Laser/BP_LaserParent.LaserColor` _laserhit) (`self.SpawnRef`) null))
          (`self.K2_AttachToComponent` _returnvalue (`self.SM_Parent`) "None" "KeepWorld" "KeepWorld" "KeepRelative" true)
          (`KismetArrayLibrary.Array_Add` (`self.LaserAttached`) _returnvalue)
          (`KismetArrayLibrary.Array_Add` (`/Game/MeinZeug/BluePrints/Laser/BPC_LaserSpawn.Child Laser` (`self.SpawnRef`)) _returnvalue)
          (return _returnvalue)
          (else
            (`self.Clear all Attached Lasers`)))))))

(fn `UserConstructionScript`
  (`parent.UserConstructionScript`))