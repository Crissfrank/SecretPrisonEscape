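; BP_EndscreenTrigger is a trigger volume that starts the game's ending when the first-person player character overlaps its box.
; On overlap it turns off the character's CanPlaySound flag, disables player input, hides the UI through the game mode and plays the referenced level sequence.
; When the sequence finishes, it creates the CAW_Ende end-screen widget, adds it to the viewport and shows the mouse cursor.
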(event `self.Box.OnComponentBeginOverlap`
  (params (OverlappedComponent :type "PrimitiveComponent Object Reference") (OtherActor :type "Actor Object Reference") (OtherComp :type "PrimitiveComponent Object Reference") (OtherBodyIndex :type Integer) (bFromSweep :type Boolean) (SweepResult :type "HitResult Structure (by ref)"))
  (bind _sequenceplayer (`LevelSequenceActor.SequencePlayer` (`self.SequenceToPlay`)))
  (bind _asbp_first_person_character (cast `/Game/FirstPerson/Blueprints/BP_FirstPersonCharacter` OtherActor))
  (set `/Game/FirstPerson/Blueprints/BP_FirstPersonCharacter.Can Play sound` false _asbp_first_person_character)
  (`self.DisableInput` (`GameplayStatics.GetPlayerCharacter` 0) (`GameplayStatics.GetPlayerController` 0))
  (bind _asbp_first_person_game_mode (cast `/Game/FirstPerson/Blueprints/BP_FirstPersonGameMode` (`GameplayStatics.GetGameMode`)))
  (`/Game/FirstPerson/Blueprints/BP_FirstPersonGameMode.Hide UI` _asbp_first_person_game_mode true)
  (`MovieSceneSequencePlayer.Play` _sequenceplayer)
  (`KismetSystemLibrary.PrintString` "Hello")
  (add `MovieSceneSequencePlayer.OnFinished` _sequenceplayer (delegate `OnFinished`)))

(event `OnFinished`
  (bind _returnvalue (`|CreateWidget` "/Game/MeinZeug/BluePrints/UI´s/CAW_Ende.CAW_Ende_C"))
  (bind _output_get (set `self.Ende` _returnvalue))
  (`UserWidget.AddToViewport` _output_get 0)
  (set `PlayerController.bShowMouseCursor` true (`GameplayStatics.GetPlayerController` 0)))

(fn `UserConstructionScript`)