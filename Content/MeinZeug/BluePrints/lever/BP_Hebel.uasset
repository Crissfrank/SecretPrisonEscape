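; Six-lever sequence puzzle that moves a BP_WandMovement wall when the levers are pulled in the correct order.
; ShowDeets stores the hit component, then RunObject uses its tag to start that lever's timeline and block re-interaction.
; Finished pulls are checked against Solution: correct ones turn their light green, while a mistake buzzes and resets raised levers to red.
; A box trigger toggles the widget's visibility.
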(event `LeverMove`
  (bind (_leverrot1_roll _leverrot1_pitch _leverrot1_yaw) (`KismetMathLibrary.BreakRotator` (`self.LeverRot1`)))
  ;[0 0 0] Lever Logic
  (if (`self.LeverUp1`)
    (set `self.LeverUp1` false)
    (bind (_direction _newtrack_0) (`Timeline|LeverMovment` :!via `ReverseFromEnd` :!label _label)
      (:`Update`
        (`SceneComponent.K2_SetRelativeRotation` (`self.Hebel`) (`KismetMathLibrary.RLerp` (`self.LeverRot1`) (`KismetMathLibrary.MakeRotator` _leverrot1_roll (- _leverrot1_pitch -80.0) _leverrot1_yaw) _newtrack_0) false false))
      (:`Finished`
        (if (`self.LeverUp1`)
          (`self.Check Solution` 1)
          (else
            (`PrimitiveComponent.SetCollisionResponseToChannel` (`self.Hebel`) "ECC_GameTraceChannel2" "ECR_Block")
            (`PrimitiveComponent.SetMaterial` (`self.Licht`) 0 "/Game/MeinZeug/Materials/LeverPuzzleMats/MI_RedEmis.MI_RedEmis")))))
    (else
      (set `self.LeverUp1` true)
      (`PrimitiveComponent.SetCollisionResponseToChannel` (`self.Hebel`) "ECC_GameTraceChannel2" "ECR_Ignore")
      (set `self.LeverRot1` (`SceneComponent.RelativeRotation` (`self.Hebel`)))
      (goto _label :!via `PlayFromStart`))))

(event `/Game/MeinZeug/BluePrints/lever/BPI_InteractLever.ShowDeets`
  (params (PlayerRef :type "/Game/FirstPerson/Blueprints/BP_FirstPersonCharacter Object Reference") (HitComponent :type "PrimitiveComponent Object Reference"))
  ;[0 0 0] Show Deets
  (set `self.Player Ref` PlayerRef)
  (set `self.Hit Component` HitComponent)
  (set `/Game/FirstPerson/Blueprints/BP_FirstPersonCharacter.IsInteractable` true (`self.Player Ref`)))

(event `Lever2Move`
  (bind (_leverrot2_roll _leverrot2_pitch _leverrot2_yaw) (`KismetMathLibrary.BreakRotator` (`self.LeverRot2`)))
  ;[0 0 0] Lever Logic
  (if (`self.LeverUp2`)
    (set `self.LeverUp2` false)
    (bind (_direction _newtrack_0) (`Timeline|Timeline` :!via `ReverseFromEnd` :!label _label_2)
      (:`Update`
        (`SceneComponent.K2_SetRelativeRotation` (`self.Hebel1`) (`KismetMathLibrary.RLerp` (`self.LeverRot2`) (`KismetMathLibrary.MakeRotator` _leverrot2_roll (- _leverrot2_pitch -80.0) _leverrot2_yaw) _newtrack_0) false false))
      (:`Finished`
        (if (`self.LeverUp2`)
          (`self.Check Solution` 2)
          (else
            (`PrimitiveComponent.SetCollisionResponseToChannel` (`self.Hebel1`) "ECC_GameTraceChannel2" "ECR_Block")
            (`PrimitiveComponent.SetMaterial` (`self.Licht2`) 0 "/Game/MeinZeug/Materials/LeverPuzzleMats/MI_RedEmis.MI_RedEmis")))))
    (else
      (set `self.LeverUp2` true)
      (`PrimitiveComponent.SetCollisionResponseToChannel` (`self.Hebel1`) "ECC_GameTraceChannel2" "ECR_Ignore")
      (set `self.LeverRot2` (`SceneComponent.RelativeRotation` (`self.Hebel1`)))
      (goto _label_2 :!via `PlayFromStart`))))

(event `ClearLever`
  ;[0 0 0] Show if its Right or Wrong
  (`GameplayStatics.PlaySound2D` "/Game/MeinZeug/SoundMusik/Sounds/Right_Wrong/user-interface-game-buzzer-false-answer-01.user-interface-game-buzzer-false-answer-01" 1.0 1.0 0.0 null null)
  (set `self.CorrectNum` 0)
  (`|ExecutionSequence`
    (:`then_0`
      (if (`self.LeverUp1`)
        (`self.LeverMove`)
        (`GameplayStatics.PlaySound2D` "/Game/MeinZeug/SoundMusik/Sounds/Hebel/object-metal-lever-twist-single-02.object-metal-lever-twist-single-02" 1.0 1.0 0.0 null null)))
    (:`then_1`
      (if (`self.LeverUp2`)
        (`self.Lever2Move`)
        (`GameplayStatics.PlaySound2D` "/Game/MeinZeug/SoundMusik/Sounds/Hebel/object-metal-lever-twist-single-02.object-metal-lever-twist-single-02" 1.0 1.0 0.0 null null)))
    (:`then_2`
      (if (`self.LeverUp3`)
        (`self.Lever3Move`)
        (`GameplayStatics.PlaySound2D` "/Game/MeinZeug/SoundMusik/Sounds/Hebel/object-metal-lever-twist-single-02.object-metal-lever-twist-single-02" 1.0 1.0 0.0 null null)))
    (:`then_3`
      (if (`self.LeverUp4`)
        (`self.Lever4Move`)
        (`GameplayStatics.PlaySound2D` "/Game/MeinZeug/SoundMusik/Sounds/Hebel/object-metal-lever-twist-single-02.object-metal-lever-twist-single-02" 1.0 1.0 0.0 null null)))
    (:`then_4`
      (if (`self.LeverUp5`)
        (`self.Lever5Move`)
        (`GameplayStatics.PlaySound2D` "/Game/MeinZeug/SoundMusik/Sounds/Hebel/object-metal-lever-twist-single-02.object-metal-lever-twist-single-02" 1.0 1.0 0.0 null null)))
    (:`then_5`
      (if (`self.LeverUp6`)
        (`self.Lever6Move`)
        (`GameplayStatics.PlaySound2D` "/Game/MeinZeug/SoundMusik/Sounds/Hebel/object-metal-lever-twist-single-02.object-metal-lever-twist-single-02" 1.0 1.0 0.0 null null)))))

(event `Lever3Move`
  (bind (_leverrot3_roll _leverrot3_pitch _leverrot3_yaw) (`KismetMathLibrary.BreakRotator` (`self.LeverRot3`)))
  ;[0 0 0] Lever Logic
  (if (`self.LeverUp3`)
    (set `self.LeverUp3` false)
    (bind (_direction _newtrack_0) (`Timeline|Timeline_0` :!via `ReverseFromEnd` :!label _label_3)
      (:`Update`
        (`SceneComponent.K2_SetRelativeRotation` (`self.Hebel2`) (`KismetMathLibrary.RLerp` (`self.LeverRot3`) (`KismetMathLibrary.MakeRotator` _leverrot3_roll (- _leverrot3_pitch -80.0) _leverrot3_yaw) _newtrack_0) false false))
      (:`Finished`
        (if (`self.LeverUp3`)
          (`self.Check Solution` 3)
          (else
            (`PrimitiveComponent.SetCollisionResponseToChannel` (`self.Hebel2`) "ECC_GameTraceChannel2" "ECR_Block")
            (`PrimitiveComponent.SetMaterial` (`self.Licht3`) 0 "/Game/MeinZeug/Materials/LeverPuzzleMats/MI_RedEmis.MI_RedEmis")))))
    (else
      (set `self.LeverUp3` true)
      (`PrimitiveComponent.SetCollisionResponseToChannel` (`self.Hebel2`) "ECC_GameTraceChannel2" "ECR_Ignore")
      (set `self.LeverRot3` (`SceneComponent.RelativeRotation` (`self.Hebel2`)))
      (goto _label_3 :!via `PlayFromStart`))))

(event `/Game/MeinZeug/BluePrints/lever/BPI_InteractLever.RunObject`
  ;[0 0 0] Run Levers Based on Tags
  (if (`ActorComponent.ComponentHasTag` (`self.Hit Component`) "H1")
    (`self.LeverMove`)
    (`GameplayStatics.PlaySound2D` "/Game/MeinZeug/SoundMusik/Sounds/Hebel/object-metal-lever-twist-single-02.object-metal-lever-twist-single-02" 1.0 1.0 0.0 null null)
    (elif (`ActorComponent.ComponentHasTag` (`self.Hit Component`) "H2")
      (`self.Lever2Move`)
      (`GameplayStatics.PlaySound2D` "/Game/MeinZeug/SoundMusik/Sounds/Hebel/object-metal-lever-twist-single-02.object-metal-lever-twist-single-02" 1.0 1.0 0.0 null null)
      (elif (`ActorComponent.ComponentHasTag` (`self.Hit Component`) "H3")
        (`self.Lever3Move`)
        (`GameplayStatics.PlaySound2D` "/Game/MeinZeug/SoundMusik/Sounds/Hebel/object-metal-lever-twist-single-02.object-metal-lever-twist-single-02" 1.0 1.0 0.0 null null)
        (elif (`ActorComponent.ComponentHasTag` (`self.Hit Component`) "H4")
          (`self.Lever4Move`)
          (`GameplayStatics.PlaySound2D` "/Game/MeinZeug/SoundMusik/Sounds/Hebel/object-metal-lever-twist-single-02.object-metal-lever-twist-single-02" 1.0 1.0 0.0 null null)
          (elif (`ActorComponent.ComponentHasTag` (`self.Hit Component`) "H5")
            (`self.Lever5Move`)
            (`GameplayStatics.PlaySound2D` "/Game/MeinZeug/SoundMusik/Sounds/Hebel/object-metal-lever-twist-single-02.object-metal-lever-twist-single-02" 1.0 1.0 0.0 null null)
            (elif (`ActorComponent.ComponentHasTag` (`self.Hit Component`) "H6")
              (`self.Lever6Move`)
              (`GameplayStatics.PlaySound2D` "/Game/MeinZeug/SoundMusik/Sounds/Hebel/object-metal-lever-twist-single-02.object-metal-lever-twist-single-02" 1.0 1.0 0.0 null null))))))))

(event `Lever4Move`
  (bind (_leverrot4_roll _leverrot4_pitch _leverrot4_yaw) (`KismetMathLibrary.BreakRotator` (`self.LeverRot4`)))
  ;[0 0 0] Lever Logic
  (if (`self.LeverUp4`)
    (set `self.LeverUp4` false)
    (bind (_direction _newtrack_0) (`Timeline|Timeline_1` :!via `ReverseFromEnd` :!label _label_4)
      (:`Update`
        (`SceneComponent.K2_SetRelativeRotation` (`self.Hebel3`) (`KismetMathLibrary.RLerp` (`self.LeverRot4`) (`KismetMathLibrary.MakeRotator` _leverrot4_roll (- _leverrot4_pitch -80.0) _leverrot4_yaw) _newtrack_0) false false))
      (:`Finished`
        (if (`self.LeverUp4`)
          (`self.Check Solution` 4)
          (else
            (`PrimitiveComponent.SetCollisionResponseToChannel` (`self.Hebel3`) "ECC_GameTraceChannel2" "ECR_Block")
            (`PrimitiveComponent.SetMaterial` (`self.Licht4`) 0 "/Game/MeinZeug/Materials/LeverPuzzleMats/MI_RedEmis.MI_RedEmis")))))
    (else
      (set `self.LeverUp4` true)
      (`PrimitiveComponent.SetCollisionResponseToChannel` (`self.Hebel3`) "ECC_GameTraceChannel2" "ECR_Ignore")
      (set `self.LeverRot4` (`SceneComponent.RelativeRotation` (`self.Hebel3`)))
      (goto _label_4 :!via `PlayFromStart`))))

(event `Lever5Move`
  (bind (_leverrot5_roll _leverrot5_pitch _leverrot5_yaw) (`KismetMathLibrary.BreakRotator` (`self.LeverRot5`)))
  ;[0 0 0] Lever Logic
  (if (`self.LeverUp5`)
    (set `self.LeverUp5` false)
    (bind (_direction _newtrack_0) (`Timeline|Timeline_2` :!via `ReverseFromEnd` :!label _label_5)
      (:`Update`
        (`SceneComponent.K2_SetRelativeRotation` (`self.Hebel4`) (`KismetMathLibrary.RLerp` (`self.LeverRot5`) (`KismetMathLibrary.MakeRotator` _leverrot5_roll (- _leverrot5_pitch -80.0) _leverrot5_yaw) _newtrack_0) false false))
      (:`Finished`
        (if (`self.LeverUp5`)
          (`self.Check Solution` 5)
          (else
            (`PrimitiveComponent.SetCollisionResponseToChannel` (`self.Hebel4`) "ECC_GameTraceChannel2" "ECR_Block")
            (`PrimitiveComponent.SetMaterial` (`self.Licht5`) 0 "/Game/MeinZeug/Materials/LeverPuzzleMats/MI_RedEmis.MI_RedEmis")))))
    (else
      (set `self.LeverUp5` true)
      (`PrimitiveComponent.SetCollisionResponseToChannel` (`self.Hebel4`) "ECC_GameTraceChannel2" "ECR_Ignore")
      (set `self.LeverRot5` (`SceneComponent.RelativeRotation` (`self.Hebel4`)))
      (goto _label_5 :!via `PlayFromStart`))))

(event `Check Solution`
  (params (Lever :type Integer))
  ;[0 0 0] Check Solution & Change color
  (bind _output_get (set `self.LeverNum` Lever))
  (if (== (`|GetArrayItem` (`self.Solution`) (`self.CorrectNum`)) _output_get)
    (set `self.CorrectNum` (+ (`self.CorrectNum`) 1))
    (switch `int` (`self.LeverNum`)
      (:`1`
        (`PrimitiveComponent.SetMaterial` (`self.Licht`) 0 "/Game/MeinZeug/Materials/LeverPuzzleMats/MI_GreenEmis.MI_GreenEmis"))
      (:`2`
        (`PrimitiveComponent.SetMaterial` (`self.Licht2`) 0 "/Game/MeinZeug/Materials/LeverPuzzleMats/MI_GreenEmis.MI_GreenEmis"))
      (:`3`
        (`PrimitiveComponent.SetMaterial` (`self.Licht3`) 0 "/Game/MeinZeug/Materials/LeverPuzzleMats/MI_GreenEmis.MI_GreenEmis"))
      (:`4`
        (`PrimitiveComponent.SetMaterial` (`self.Licht4`) 0 "/Game/MeinZeug/Materials/LeverPuzzleMats/MI_GreenEmis.MI_GreenEmis"))
      (:`5`
        (`PrimitiveComponent.SetMaterial` (`self.Licht5`) 0 "/Game/MeinZeug/Materials/LeverPuzzleMats/MI_GreenEmis.MI_GreenEmis"))
      (:`6`
        (`PrimitiveComponent.SetMaterial` (`self.Licht6`) 0 "/Game/MeinZeug/Materials/LeverPuzzleMats/MI_GreenEmis.MI_GreenEmis")))
    (if (== (`self.CorrectNum`) 6)
      (`GameplayStatics.PlaySound2D` "/Game/MeinZeug/SoundMusik/Sounds/Right_Wrong/object-metal-bicycle-bell-ring-01.object-metal-bicycle-bell-ring-01" 1.0 1.0 0.0 null null)
      (bind _asbp_wand_movement (cast `/Game/MeinZeug/BluePrints/lever/BP_WandMovement` (`self.MoveWall`)))
      (`/Game/MeinZeug/BluePrints/lever/BP_WandMovement.MoveWall` _asbp_wand_movement))
    (else
      (`self.ClearLever`))))

(event `Lever6Move`
  (bind (_leverrot6_roll _leverrot6_pitch _leverrot6_yaw) (`KismetMathLibrary.BreakRotator` (`self.LeverRot6`)))
  ;[0 0 0] Lever Logic
  (if (`self.LeverUp6`)
    (set `self.LeverUp6` false)
    (bind (_direction _newtrack_0) (`Timeline|Timeline_3` :!via `ReverseFromEnd` :!label _label_6)
      (:`Update`
        (`SceneComponent.K2_SetRelativeRotation` (`self.Hebel5`) (`KismetMathLibrary.RLerp` (`self.LeverRot6`) (`KismetMathLibrary.MakeRotator` _leverrot6_roll (- _leverrot6_pitch -80.0) _leverrot6_yaw) _newtrack_0) false false))
      (:`Finished`
        (if (`self.LeverUp6`)
          (`self.Check Solution` 6)
          (else
            (`PrimitiveComponent.SetCollisionResponseToChannel` (`self.Hebel5`) "ECC_GameTraceChannel2" "ECR_Block")
            (`PrimitiveComponent.SetMaterial` (`self.Licht6`) 0 "/Game/MeinZeug/Materials/LeverPuzzleMats/MI_RedEmis.MI_RedEmis")))))
    (else
      (set `self.LeverUp6` true)
      (`PrimitiveComponent.SetCollisionResponseToChannel` (`self.Hebel5`) "ECC_GameTraceChannel2" "ECR_Ignore")
      (set `self.LeverRot6` (`SceneComponent.RelativeRotation` (`self.Hebel5`)))
      (goto _label_6 :!via `PlayFromStart`))))

(event `self.Box.OnComponentBeginOverlap`
  (params (OverlappedComponent :type "PrimitiveComponent Object Reference") (OtherActor :type "Actor Object Reference") (OtherComp :type "PrimitiveComponent Object Reference") (OtherBodyIndex :type Integer) (bFromSweep :type Boolean) (SweepResult :type "HitResult Structure (by ref)"))
  (`SceneComponent.SetHiddenInGame` (`self.Widget`) false false))

(event `self.Box.OnComponentEndOverlap`
  (params (OverlappedComponent :type "PrimitiveComponent Object Reference") (OtherActor :type "Actor Object Reference") (OtherComp :type "PrimitiveComponent Object Reference") (OtherBodyIndex :type Integer))
  (`SceneComponent.SetHiddenInGame` (`self.Widget`) true false))

(fn `UserConstructionScript`)